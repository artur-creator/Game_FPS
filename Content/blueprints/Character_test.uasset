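; Test player character for a shooter, with movement, look, jump, sprint, shooting and reloading.
; On BeginPlay it spawns a rifle, attaches it to the Weapon component and creates the HUD widget.
; Holding the shot axis fires repeatedly along the camera's forward vector, gated by a CanShoot flag and a fire-rate Delay.
; Shooting and reloading are delegated to the equipped gun, then update the HUD ammo from its magazine.
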(event `self.ReceiveBeginPlay`
  (bind _weapon (`self.Weapon`))
  (bind _returnvalue (`|SpawnActorFromClass` "/Game/blueprints/rifle_blueprint.rifle_blueprint_C" (`SceneComponent.K2_GetComponentToWorld` _weapon) "Undefined" "MultiplyWithRoot" null null))
  (bind _output_get (set `self.equiped_gun` _returnvalue))
  (`self.K2_AttachToComponent` _output_get _weapon "None" "SnapToTarget" "SnapToTarget" "KeepRelative" true)
  (bind _returnvalue_2 (`|CreateWidget` "/Game/blueprints/player_hud_test.player_hud_test_C"))
  (`UserWidget.AddToViewport` _returnvalue_2 0)
  (set `self.hud` _returnvalue_2))

(event `InputAxis|forward`
  (params (AxisValue :type "Float (single-precision)"))
  (`self.AddMovementInput` (`self.GetActorForwardVector`) AxisValue))

(event `InputAxis|shot`
  (params (AxisValue :type "Float (single-precision)"))
  (bind _camera (`self.Camera`))
  (bind _returnvalue (`SceneComponent.K2_GetComponentLocation` _camera))
  (if (and (== AxisValue 1.0) (`self.can_shoot`))
    (`/Game/blueprints/weapon_base.shoot` (`self.equiped_gun`) _returnvalue (+ _returnvalue (* (`SceneComponent.GetForwardVector` _camera) (`/Game/blueprints/weapon_base.max_dist` (`self.equiped_gun`)))))
    (`/Game/blueprints/player_hud_test.update_ammo` (`self.hud`) (`/Game/blueprints/weapon_base.magaz` (`self.equiped_gun`)))
    (set `self.can_shoot` false)
    (`KismetSystemLibrary.Delay` (`/Game/blueprints/weapon_base.fire_rate` (`self.equiped_gun`)))
    (set `self.can_shoot` true)))

(event `InputAxis|right`
  (params (AxisValue :type "Float (single-precision)"))
  (`self.AddMovementInput` (`self.GetActorRightVector`) AxisValue))

(event `InputAxis|look_x`
  (params (AxisValue :type "Float (single-precision)"))
  (`self.AddControllerYawInput` AxisValue))

(event `InputAction|reload`
  (params (Key :type "Key Structure"))
  (:`Pressed`
    (`/Game/blueprints/weapon_base.reload` (`self.equiped_gun`) 30)
    (`/Game/blueprints/player_hud_test.update_ammo` (`self.hud`) (`/Game/blueprints/weapon_base.magaz` (`self.equiped_gun`)))))

(event `InputAxis|look_y`
  (params (AxisValue :type "Float (single-precision)"))
  (`self.AddControllerPitchInput` (* AxisValue -1.0)))

(event `InputAction|jump`
  (params (Key :type "Key Structure"))
  (:`Pressed`
    (`self.Jump`)))

(event `InputAction|run`
  (params (Key :type "Key Structure"))
  (:`Pressed`
    (set `CharacterMovementComponent.MaxWalkSpeed` 3000.0 (`self.CharacterMovement`)))
  (:`Released`
    (set `CharacterMovementComponent.MaxWalkSpeed` 600.0 (`self.CharacterMovement`))))

(fn `UserConstructionScript`)