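; Base weapon Blueprint providing hitscan shooting and magazine reloading, with no active event logic of its own.
; Shoot spends a round if any remain, plays a sound at the weapon and line-traces the Visibility channel between caller-supplied points.
; A hit spawns the Burst effect at the impact location and applies Damage to the hit actor.
; Reload sets the magazine to the given amount, capped at MaxBullets, rather than adding to it.
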(fn `reload`
  (params (amount :type Integer))
  (bind _max_bullets (`self.max_bullets`))
  (if (< amount _max_bullets)
    (set `self.magaz` amount)
    (else
      (set `self.magaz` _max_bullets))))

(fn `shoot`
  (params (Start :type "Vector Structure") (End :type "Vector Structure"))
  (if (> (`self.magaz`) 0)
    (set `self.magaz` (- (`self.magaz`) 1))
    (`GameplayStatics.PlaySoundAtLocation` (`self.sound`) (`KismetMathLibrary.TransformLocation` (`self.GetTransform`)) (struct) 1.0 1.0 0.0 null null null null)
    (bind (_outhit _returnvalue) (`KismetSystemLibrary.LineTraceSingle` Start End "TraceTypeQuery1"))
    (if _returnvalue
      (bind (_bblockinghit _binitialoverlap _time _distance _location _impactpoint _normal _impactnormal _physmat _hitactor) (`GameplayStatics.BreakHitResult` _outhit))
      (`NiagaraFunctionLibrary.SpawnSystemAtLocation` (`self.burst`) _location)
      (`GameplayStatics.ApplyDamage` _hitactor (`self.damage`)))))

(fn `UserConstructionScript`)